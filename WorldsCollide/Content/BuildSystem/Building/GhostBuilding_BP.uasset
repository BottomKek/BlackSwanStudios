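; GhostBuilding_BP is the placeholder actor that stands in for a building during construction in the build system.
; On BeginPlay it takes its mesh from ConstructionInfo, applies the BasicAsset01 material and starts a timer for the build time.
; When the timer fires, it spawns the building class from ConstructionInfo at its own transform, prints a completion message and destroys itself.
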(event `self.ReceiveBeginPlay`
  (bind (_mesh _buildtime) (break `/Game/BuildSystem/Building/ConstructionInfo` (`self.ConstructionInfo`)))
  (`StaticMeshComponent.SetStaticMesh` (`self.StaticMesh`) _mesh)
  (`PrimitiveComponent.SetMaterial` (`self.StaticMesh`) 0 "/Engine/MapTemplates/Materials/BasicAsset01.BasicAsset01")
  (`KismetSystemLibrary.K2_SetTimerDelegate` (delegate `ReplaceWithBuilding`) _buildtime))

(event `ReplaceWithBuilding`
  (bind (_constructioninfo_mesh _constructioninfo_buildtime _constructioninfo_buildreference) (break `/Game/BuildSystem/Building/ConstructionInfo` (`self.ConstructionInfo`)))
  (`|SpawnActorFromClass` _constructioninfo_buildreference (`self.GetTransform`) "Undefined" "MultiplyWithRoot" null null)
  (`KismetSystemLibrary.PrintString` "Build Complete")
  (`self.K2_DestroyActor`))

(fn `UserConstructionScript`)