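; Construction manager that lets the player place buildings with the mouse through a ghost preview.
; On BeginPlay it creates the construction test UI and registers itself with that widget and the camera controller.
; SpawnBuilding spawns a ghost carrying construction info, which Tick moves to a grid-snapped cursor trace hit.
; A short timer, or calling SpawnBuilding again, ends placement by releasing the ghost reference.
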(event `self.ReceiveBeginPlay`
  (bind _returnvalue (`GameplayStatics.GetPlayerController` 0))
  ;[1 1 1] Set up the UI so the player can place buildings
  (`|ExecutionSequence`
    (:`then_0`
      (set `PlayerController.bShowMouseCursor` true _returnvalue)
      (`WidgetBlueprintLibrary.SetInputMode_GameAndUIEx` _returnvalue null)
      (bind _returnvalue_2 (`|CreateWidget` "/Game/BuildSystem/Construction/ConstructionTestUI.ConstructionTestUI_C" _returnvalue))
      (`UserWidget.AddToViewport` _returnvalue_2 0)
      (set `/Game/BuildSystem/Construction/ConstructionTestUI.ConstructionManager` self _returnvalue_2))
    (:`then_1`
      (bind _asbp_camera_controller (cast `/Game/Controls/BP_CameraController` (`GameplayStatics.GetPlayerController` 0)))
      (set `/Game/Controls/BP_CameraController.ConstructionManagerRef` self _asbp_camera_controller))))

(event `Spawn Building`
  (params (`To Build` :type "/Game/BuildSystem/Building/Building_Master_BP Class Reference"))
  ;[1 1 1] Spawn the Ghost of the Building that will eventually become building.
  (if (`self.ActivePlacement`)
    (set `self.ActiveGhostBuilding` null)
    (set `self.ActivePlacement` false)
    (else
      (set `self.ActivePlacement` true)
      (bind _returnvalue (`|SpawnActorFromClass` "/Game/BuildSystem/Building/GhostBuilding_BP.GhostBuilding_BP_C" (`KismetMathLibrary.MakeTransform` (0.0 0.0 0.0)) "Undefined" "MultiplyWithRoot" null (make `/Game/BuildSystem/Building/ConstructionInfo` null 5.0 `To Build`) null))
      (set `self.ActiveGhostBuilding` _returnvalue)
      (`KismetSystemLibrary.K2_SetTimerDelegate` (delegate `Finalize Plaecement`) 2.0))))

(event `Finalize Plaecement`
  (set `self.ActivePlacement` false)
  (set `self.ActiveGhostBuilding` null))

(event `self.ReceiveTick`
  (params (DeltaSeconds :type "Float (single-precision)"))
  (bind (_worldlocation _worlddirection) (`PlayerController.DeprojectMousePositionToWorld` (`GameplayStatics.GetPlayerController` 0)))
  ;[1 1 1] Get the Location of the Mouse in the world and move the ghost building there.
  (if (`self.ActivePlacement`)
    (bind _outhit (`KismetSystemLibrary.LineTraceSingle` _worldlocation (* _worlddirection 10000.0) "TraceTypeQuery1"))
    (bind (_returnvalue_x _returnvalue_y) (`KismetMathLibrary.BreakVector` (`KismetMathLibrary.Vector_SnappedToGrid` (`.Location` (`GameplayStatics.BreakHitResult` _outhit)) (`self.GridSize`))))
    (`self.K2_SetActorLocation` (`self.ActiveGhostBuilding`) (`KismetMathLibrary.MakeVector` _returnvalue_x _returnvalue_y) false false)))

(fn `UserConstructionScript`)