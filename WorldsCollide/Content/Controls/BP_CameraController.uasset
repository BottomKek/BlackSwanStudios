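; Camera controller that pans the player pawn with directional Enhanced Input actions and screen-edge mouse scrolling, with the cursor visible and locked to the viewport.
; DoOnce-gated key events build CameraMovement, which MoveCamera merges with mouse-edge offsets, normalizes and applies every Tick without delta time.
; CameraZoom, never set here, interpolates speed and pitch at fixed yaw.
; Grid-bound clamps and a placement-finalize call are left unconnected.
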(event `self.ReceiveTick`
  (params (DeltaSeconds :type "Float (single-precision)"))
  (`self.MoveCamera`))

(event `self.ReceiveBeginPlay`
  (bind _returnvalue (`GameplayStatics.GetPlayerController` 0))
  (bind _returnvalue_2 (pcsubsystem `EnhancedInputLocalPlayerSubsystem` self))
  (set `self.CameraPawn` (`GameplayStatics.GetPlayerPawn` 0))
  (`/Engine/EditorBlueprintResources/StandardMacros.IsValid` _returnvalue_2
    (:`Is Valid`
      (`EnhancedInputSubsystemInterface.AddMappingContext` _returnvalue_2 "/Game/Controls/IMC_Controls.IMC_Controls" 0 (struct))
      (`WidgetBlueprintLibrary.SetInputMode_GameAndUIEx` _returnvalue null "LockAlways" false)
      (set `PlayerController.bShowMouseCursor` true _returnvalue))))

(event `EnhancedInput|/Game/Controls/IA_CameraUp`
  (params (ActionValue :type Boolean) (ElapsedSeconds :type "Float (double-precision)") (TriggeredSeconds :type "Float (double-precision)") (InputAction :type "InputAction Object Reference" :default "/Game/Controls/IA_CameraUp.IA_CameraUp"))
  (bind _cameramovement (`self.CameraMovement`))
  (:`Triggered`
    (`/Engine/EditorBlueprintResources/StandardMacros.DoOnce` false :!label _label
      (:`Completed`
        (set `self.CameraMovement` (+ _cameramovement (0.0 -1.0 0.0))))))
  (:`Completed`
    (set `self.CameraMovement` (- _cameramovement (0.0 -1.0 0.0)))
    (goto _label :!via `Reset`)))

(event `EnhancedInput|/Game/Controls/IA_CameraDown`
  (params (ActionValue :type Boolean) (ElapsedSeconds :type "Float (double-precision)") (TriggeredSeconds :type "Float (double-precision)") (InputAction :type "InputAction Object Reference" :default "/Game/Controls/IA_CameraDown.IA_CameraDown"))
  (bind _cameramovement (`self.CameraMovement`))
  (:`Triggered`
    (`/Engine/EditorBlueprintResources/StandardMacros.DoOnce` false :!label _label_2
      (:`Completed`
        (set `self.CameraMovement` (+ _cameramovement (0.0 1.0 0.0))))))
  (:`Completed`
    (set `self.CameraMovement` (- _cameramovement (0.0 1.0 0.0)))
    (goto _label_2 :!via `Reset`)))

(event `EnhancedInput|/Game/Controls/IA_CameraRight`
  (params (ActionValue :type Boolean) (ElapsedSeconds :type "Float (double-precision)") (TriggeredSeconds :type "Float (double-precision)") (InputAction :type "InputAction Object Reference" :default "/Game/Controls/IA_CameraRight.IA_CameraRight"))
  (bind _cameramovement (`self.CameraMovement`))
  (:`Triggered`
    (`/Engine/EditorBlueprintResources/StandardMacros.DoOnce` false :!label _label_3
      (:`Completed`
        (set `self.CameraMovement` (+ _cameramovement (1.0 0.0 0.0))))))
  (:`Completed`
    (set `self.CameraMovement` (- _cameramovement (1.0 0.0 0.0)))
    (goto _label_3 :!via `Reset`)))

(event `EnhancedInput|/Game/Controls/IA_CameraLeft`
  (params (ActionValue :type Boolean) (ElapsedSeconds :type "Float (double-precision)") (TriggeredSeconds :type "Float (double-precision)") (InputAction :type "InputAction Object Reference" :default "/Game/Controls/IA_CameraLeft.IA_CameraLeft"))
  (bind _cameramovement (`self.CameraMovement`))
  (:`Triggered`
    (`/Engine/EditorBlueprintResources/StandardMacros.DoOnce` false :!label _label_4
      (:`Completed`
        (set `self.CameraMovement` (+ _cameramovement (-1.0 0.0 0.0))))))
  (:`Completed`
    (set `self.CameraMovement` (- _cameramovement (-1.0 0.0 0.0)))
    (goto _label_4 :!via `Reset`)))

(fn `MoveCamera`
  (bind (_sizex _sizey) (`self.GetViewportSize`))
  (bind _sizex_2 (`self.GetViewportSize`))
  (bind _camerapawn (`self.CameraPawn`))
  (bind (_returnvalue_x _returnvalue_y _returnvalue_z) (`KismetMathLibrary.BreakVector` (+ (`self.K2_GetActorLocation` _camerapawn) (* (`KismetMathLibrary.Normal` (- (`KismetMathLibrary.Normal` (`self.CameraMovement`)) (`KismetMathLibrary.MakeVector` (- 1.0 (`KismetMathLibrary.FClamp` (`KismetMathLibrary.NormalizeToRange` (`self.MouseX`) 0.0 (* (`self.GetViewportSize`) 0.05))))) (`KismetMathLibrary.MakeVector` (* -1.0 (`KismetMathLibrary.FClamp` (`KismetMathLibrary.NormalizeToRange` (`self.MouseX`) (* _sizex_2 0.95) (`KismetMathLibrary.Conv_IntToDouble` _sizex_2))))) (`KismetMathLibrary.MakeVector` 0.0 (- 1.0 (`KismetMathLibrary.FClamp` (`KismetMathLibrary.NormalizeToRange` (`self.MouseY`) 0.0 (* (`.SizeY` (`self.GetViewportSize`)) 0.05))))) (`KismetMathLibrary.MakeVector` 0.0 (* -1.0 (`KismetMathLibrary.FClamp` (`KismetMathLibrary.NormalizeToRange` (`self.MouseY`) (* _sizey 0.95) (`KismetMathLibrary.Conv_IntToDouble` _sizey))))))) (`KismetMathLibrary.Lerp` (`self.MinCameraSpeed`) (`self.MaxCameraSpeed`) (`self.CameraZoom`))))))
  (bind _returnvalue (`WidgetLayoutLibrary.GetMousePositionOnViewport`))
  (set `self.MouseX` (`KismetMathLibrary.BreakVector2D` _returnvalue))
  (set `self.MouseY` (`.Y` (`KismetMathLibrary.BreakVector2D` _returnvalue)))
  (`self.K2_SetActorLocationAndRotation` _camerapawn (`KismetMathLibrary.MakeVector` _returnvalue_x _returnvalue_y _returnvalue_z) (`KismetMathLibrary.MakeRotator` 0.0 (`KismetMathLibrary.Lerp` 15.0 0.0 (`self.CameraZoom`)) -90.0) false false))

(fn `UserConstructionScript`)