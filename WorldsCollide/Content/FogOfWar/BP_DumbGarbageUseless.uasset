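; Abandoned fog of war actor, marked by its own comment as a naive, performance-heavy approach.
; Its construction script calls PlaceFog, but that event is empty, so no fog is placed.
; Disconnected logic would clear ISMFog and fill a grid, sized by GridSize and GapSize, with one raised world-space instance per cell.
; That logic multiplies actor location by the cell offset rather than adding it.
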(event `PlaceFog`)

(fn `UserConstructionScript`
  (`self.PlaceFog`))